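; Sword weapon Blueprint with a GrabComponent; its BeginPlay, overlap and Tick events and its construction script are all empty.
; The event graph holds only disconnected debug chains that would nudge the GrabComponent's relative roll, pitch or yaw in fixed steps either way and print the rotation, apparently for tuning grip orientation.
; None of these chains has a trigger, so the graph does nothing at runtime.
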(event EventBeginPlay)

(event Collision|EventActorBeginOverlap
  (params (OtherActor :type Actor%20Object%20Reference)))

(event EventTick
  (params (DeltaSeconds :type Float%20%28single-precision%29)))

(event Input|KeyboardEvents|DebugKeyQ
  (params (Key :type Key%20Structure :default "None") (ActionValue :type Input%20Action%20Value%20Structure)))

(event Input|KeyboardEvents|DebugKeyW
  (params (Key :type Key%20Structure :default "None") (ActionValue :type Input%20Action%20Value%20Structure)))

(event Input|KeyboardEvents|DebugKeyA
  (params (Key :type Key%20Structure :default "None") (ActionValue :type Input%20Action%20Value%20Structure)))

(event Input|KeyboardEvents|DebugKeyS
  (params (Key :type Key%20Structure :default "None") (ActionValue :type Input%20Action%20Value%20Structure)))

(event Input|KeyboardEvents|DebugKeyZ
  (params (Key :type Key%20Structure :default "None") (ActionValue :type Input%20Action%20Value%20Structure)))

(event Input|KeyboardEvents|DebugKeyX
  (params (Key :type Key%20Structure :default "None") (ActionValue :type Input%20Action%20Value%20Structure)))

(fn ConstructionScript)